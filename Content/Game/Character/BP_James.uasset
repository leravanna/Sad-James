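; BP_James is the player character, with Enhanced Input for looking, moving, aiming and running.
; Look yaws the controller and pitches the spring arm within clamped limits, while aiming switches rotation from movement-oriented to controller-driven and running toggles walk speed.
; An idle timer sets a sad state after a few seconds without activity.
; Debug-style E and F keys set and print the weapon flag in BP_GameInstance, while EquipWeapon is empty.
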(event `self.ReceiveBeginPlay`
  (bind _returnvalue (pcsubsystem `EnhancedInputLocalPlayerSubsystem` (`GameplayStatics.GetPlayerController` 0)))
  ; Add IMC
  (`/Engine/EditorBlueprintResources/StandardMacros.IsValid` _returnvalue
    (:`Is Valid`
      (`EnhancedInputSubsystemInterface.AddMappingContext` _returnvalue "/Game/Game/Inputs/IMC_James.IMC_James" 0 (struct))
      (`self.Stop Aiming`))))

(event `EnhancedInput|/Game/Game/Inputs/Actions/IA_Look`
  (params (ActionValue :type "Vector2D Structure") (ElapsedSeconds :type "Float (double-precision)") (TriggeredSeconds :type "Float (double-precision)") (InputAction :type "InputAction Object Reference" :default "/Game/Game/Inputs/Actions/IA_Look.IA_Look"))
  (bind (_x _y) (`KismetMathLibrary.BreakVector2D` ActionValue))
  ; View
  (:`Triggered`
    (`self.AddControllerYawInput` _x)
    (bind _output_get (set `self.Vertical Angle` (`KismetMathLibrary.ClampAngle` (+ (`self.Vertical Angle`) _y) -60.0 60.0)))
    (`SceneComponent.K2_SetRelativeRotation` (`self.SpringArm`) (`KismetMathLibrary.MakeRotator` 0.0 _output_get) false false)
    (`self.Start Doing Something`))
  (:`Completed`
    (`self.Doing Nothing`)))

(event `EnhancedInput|/Game/Game/Inputs/Actions/IA_Move`
  (params (ActionValue :type "Vector2D Structure") (ElapsedSeconds :type "Float (double-precision)") (TriggeredSeconds :type "Float (double-precision)") (InputAction :type "InputAction Object Reference" :default "/Game/Game/Inputs/Actions/IA_Move.IA_Move"))
  (bind _returnvalue (`self.GetControlRotation`))
  (bind (_x _y) (`KismetMathLibrary.BreakVector2D` ActionValue))
  ; Move
  (:`Triggered`
    (`self.AddMovementInput` (+ (* _x (`KismetMathLibrary.GetForwardVector` _returnvalue)) (* _y (`KismetMathLibrary.GetRightVector` _returnvalue))))
    (`self.Start Doing Something`))
  (:`Completed`
    (`self.Doing Nothing`)))

(event `EnhancedInput|/Game/Game/Inputs/Actions/IA_Aim`
  (params (ActionValue :type Boolean) (ElapsedSeconds :type "Float (double-precision)") (TriggeredSeconds :type "Float (double-precision)") (InputAction :type "InputAction Object Reference" :default "/Game/Game/Inputs/Actions/IA_Aim.IA_Aim"))
  ; Aim
  (:`Started`
    (`self.Start Aiming`)
    (`KismetSystemLibrary.PrintString` "Aim started"))
  (:`Completed`
    (`self.Stop Aiming`)
    (`KismetSystemLibrary.PrintString` "Aim Completed")
    (`self.Doing Nothing`)))

(event `Start Aiming`
  (bind _charactermovement (`self.CharacterMovement`))
  ; Start Aiming
  (set `CharacterMovementComponent.bOrientRotationToMovement` false _charactermovement)
  (set `CharacterMovementComponent.bUseControllerDesiredRotation` true _charactermovement)
  (set `self.Is Aiming` true)
  (`self.Start Doing Something`))

(event `Stop Aiming`
  (bind _charactermovement (`self.CharacterMovement`))
  ; Stop Aiming
  (set `CharacterMovementComponent.bOrientRotationToMovement` true _charactermovement)
  (set `CharacterMovementComponent.bUseControllerDesiredRotation` false _charactermovement)
  (set `self.Is Aiming` false))

(event `EnhancedInput|/Game/Game/Inputs/Actions/IA_Run`
  (params (ActionValue :type Boolean) (ElapsedSeconds :type "Float (double-precision)") (TriggeredSeconds :type "Float (double-precision)") (InputAction :type "InputAction Object Reference" :default "/Game/Game/Inputs/Actions/IA_Run.IA_Run"))
  (:`Started`
    (set `self.Is Running` true)
    (`self.Update Character Speed` :!label _label))
  (:`Canceled`
    (set `self.Is Running` false :!label _label_2)
    (goto _label))
  (:`Completed`
    (goto _label_2)))

(event `Start Doing Something`
  ; James is Sad
  (set `self.IsDoingNothing` false)
  (set `self.Is Sad` false)
  (`KismetSystemLibrary.K2_ClearAndInvalidateTimerHandle` (`self.DoingNothingHandle`)))

(event `Start being Sad`
  ; James is Sad
  (set `self.Is Sad` true))

(event `Doing Nothing`
  ; James is Sad
  (if (not (`self.IsDoingNothing`))
    (set `self.IsDoingNothing` true)
    (bind _returnvalue (`KismetSystemLibrary.K2_SetTimerDelegate` (delegate `Start being Sad`) 4.0))
    (set `self.DoingNothingHandle` _returnvalue)))

(event `Key|F`
  (params (Key :type "Key Structure"))
  (:`Pressed`
    (bind _asbp_game_instance (cast `/Game/Game/Blueprints/BP_GameInstance` (`GameplayStatics.GetGameInstance`)))
    (if (`/Game/Game/Blueprints/BP_GameInstance.Has Weapon` _asbp_game_instance)
      (`KismetSystemLibrary.PrintString` "James has weapon")
      (else
        (`KismetSystemLibrary.PrintString` "James doesnt have a weapon")))))

(event `Key|E`
  (params (Key :type "Key Structure"))
  (:`Pressed`
    (bind _asbp_game_instance (cast `/Game/Game/Blueprints/BP_GameInstance` (`GameplayStatics.GetGameInstance`)))
    (set `/Game/Game/Blueprints/BP_GameInstance.Has Weapon` true _asbp_game_instance)))

(event `Equip Weapon`)

(fn `Update Character Speed`
  (if (`self.Is Running`)
    (set `CharacterMovementComponent.MaxWalkSpeed` 400.0 (`self.CharacterMovement`))
    (else
      (set `CharacterMovementComponent.MaxWalkSpeed` 120.0 (`self.CharacterMovement`)))))

(fn `UserConstructionScript`
  (`self.Update Character Speed`))